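; Padlocked double gate for Ana's labyrinth minigame that toggles between open and closed.
; Construction script orients it horizontally or vertically and picks the padlock mesh and dynamic material from GateIndex.
; IsClosed sets the box to overlap or ignore a custom trace channel and drives the animation.
; Timelines float the padlock in a loop, fade it and swing the mirrored leaves, with delays reversing their order on closing.
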(event Custom|switchOpenClose
  ;[1 0.4411 0.7244 0.5] switchOpenClose
  (Variables|Default|SetisClosed (not (Variables|Default|GetisClosed))) ; switch its previous value
  ;;[1 0.4411 0.7244 0.5] set collision depending on open or closed
  (Collision|SetCollisionResponsetoChannel (Variables|Default|GetBox) "ECC_GameTraceChannel2" (select (Variables|Default|GetisClosed) "ECR_Overlap" "ECR_Ignore"))
  (CallFunction|OpenCloseGateAnimation (not (Variables|Default|GetisClosed))))

(event Custom|candadoeFloatee
  (bind _candadoe (Variables|Default|Getcandadoe))
  (bind _relativelocation (Variables|/Script/Engine.SceneComponent|GetRelativeLocation _candadoe))
  ;[1 0.4873 0.5131 0.5] candadoe floatee
  (Utilities|FlowControl|Sequence
    (:then_0
      (Components|Timeline|SetPlayRate (Variables|Default|GetTimeline) 0.3)
      (bind _newtrack_0 (Timeline|Timeline PlayFromStart)
        (:Update
          (Transformation|SetRelativeLocation (Variables|Default|Getcandadoe) (Math|Vector|MakeVector (Math|Float|Lerp -15.0 1e+01 _newtrack_0) (.y _relativelocation) (.z _relativelocation)) false false))
        (:Finished
          (Timeline|Timeline PlayFromStart))))))

(event Custom|openCloseGateAnimation
  (params (trueMeansOpen :type Boolean))
  ;[0.51 1 0.5255 0.5] open lock animation
  (Utilities|FlowControl|Sequence
    (:then_0
      (Utilities|FlowControl|Delay (select trueMeansOpen 0.0 0.4))
      (Components|Timeline|SetPlayRate (Variables|Default|GetgateOpen) 1.0)
      (if trueMeansOpen
        (bind _newtrack_0 (Timeline|candadoeFadeInOut PlayFromStart)
          (:Update
            (Rendering|Material|SetScalarParameterValue (Variables|Default|GetcandadoeMaterial) "Block Opacity" _newtrack_0 :!class /Script/Engine.MaterialInstanceDynamic)))
        (else
          (Timeline|candadoeFadeInOut ReverseFromEnd))))
    (:then_1
      (Utilities|FlowControl|Delay (select trueMeansOpen 0.4 0.0))
      (Components|Timeline|SetPlayRate (Variables|Default|GetgateOpen) 1.5)
      (if trueMeansOpen
        (bind _newtrack_0_2 (Timeline|gateOpen PlayFromStart)
          (:Update
            (Transformation|SetRelativeRotation (Variables|Default|GetgateMesh) (Math|Rotator|MakeRotator 0.0 0.0 (Math|Float|Lerp 0.0 9e+01 _newtrack_0_2)) false false)
            (Transformation|SetRelativeRotation (Variables|Default|GetgateMesh1) (Math|Rotator|MakeRotator 0.0 0.0 (* (Math|Float|Lerp 0.0 9e+01 _newtrack_0_2) -1.0)) false false)))
        (else
          (Timeline|gateOpen ReverseFromEnd))))))

(event Custom|beginPlayOpenClose
  ;[1 0.4411 0.7244 0.5] switchOpenClose
  ;;[1 0.4411 0.7244 0.5] set collision depending on open or closed
  (Collision|SetCollisionResponsetoChannel (Variables|Default|GetBox) "ECC_GameTraceChannel2" (select (Variables|Default|GetisClosed) "ECR_Overlap" "ECR_Ignore"))
  (CallFunction|OpenCloseGateAnimation (not (Variables|Default|GetisClosed))))

(event EventPrepareCollisions
  ;[1 0.4719 0 0.5] prepareCollisionsOverride
  ;;[1 0.3842 0.002751 0.5] set collision depending on open or closed
  (Collision|SetCollisionResponsetoChannel (Variables|Default|GetBox) "ECC_GameTraceChannel2" (select (Variables|Default|GetisClosed) "ECR_Overlap" "ECR_Ignore"))
  (CallFunction|CandadoeFloatee)
  (CallFunction|BeginPlayOpenClose))

(fn ConstructionScript
  (bind _candadoe (Variables|Default|Getcandadoe))
  (|CallParentFunction)
  ;[1 1 1 0.5] rotate the gate root depending on the boolean
  (Transformation|SetRelativeRotation (Variables|Default|GetgateRoot) (select (Variables|Default|GetisHorizontal) "0, 0, 0" "0.000000,90.000000,0.000000") false false)
  (Components|StaticMesh|SetStaticMesh _candadoe (Utilities|Select :Index (Variables|Default|GetgateIndex) :Option%200 "/Game/Art/Minigames/Ana/SM_AnaLabyrinth_Padlock_04.SM_AnaLabyrinth_Padlock_04" :Option%201 "/Game/Art/Minigames/Ana/SM_AnaLabyrinth_Padlock_01.SM_AnaLabyrinth_Padlock_01" :Option%202 "/Game/Art/Minigames/Ana/SM_AnaLabyrinth_Padlock_02.SM_AnaLabyrinth_Padlock_02" :Option%203 "/Game/Art/Minigames/Ana/SM_AnaLabyrinth_Padlock_03.SM_AnaLabyrinth_Padlock_03" :Option%204 "/Game/Art/Minigames/Ana/SM_AnaLabyrinth_Padlock_04.SM_AnaLabyrinth_Padlock_04"))
  (bind _returnvalue (Rendering|Material|CreateDynamicMaterialInstance _candadoe 0 (Utilities|Select :Index (Variables|Default|GetgateIndex) :Option%200 "/Game/Art/Minigames/Ana/MI_AnaLabyrinth_Larntern_Padlocks04.MI_AnaLabyrinth_Larntern_Padlocks04" :Option%201 "/Game/Art/Minigames/Ana/MI_AnaLabyrinth_Larntern_Padlocks01.MI_AnaLabyrinth_Larntern_Padlocks01" :Option%202 "/Game/Art/Minigames/Ana/MI_AnaLabyrinth_Larntern_Padlocks02.MI_AnaLabyrinth_Larntern_Padlocks02" :Option%203 "/Game/Art/Minigames/Ana/MI_AnaLabyrinth_Larntern_Padlocks03.MI_AnaLabyrinth_Larntern_Padlocks03" :Option%204 "/Game/Art/Minigames/Ana/MI_AnaLabyrinth_Larntern_Padlocks04.MI_AnaLabyrinth_Larntern_Padlocks04") "None" :!class /Script/Engine.PrimitiveComponent))
  (Variables|Default|SetcandadoeMaterial _returnvalue))