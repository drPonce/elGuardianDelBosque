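; Button actor for the Ana labyrinth minigame that shows a pressed or unpressed look for its gate.
; The construction script picks the button mesh and unpressed material from GateIndex, with index 0 sharing the variant 4 assets.
; Each switchBetweenPressedAndUnpressed call alternates the material through a FlipFlop and plays the matching on or off sound via the player controller's sound controller.
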(event Custom|switchBetweenPressedAndUnpressed
  (bind _isa (Utilities|FlowControl|FlipFlop)
    (:A
      _)
    (:B
      _))
  (Rendering|Material|SetMaterial (Variables|Default|Getbutton) 0 (select _isa (Utilities|Select :Index (Variables|Default|GetgateIndex) :Option%200 "/Game/Art/Minigames/Ana/MI_AnaLabyrinth_Button_04_Pressed.MI_AnaLabyrinth_Button_04_Pressed" :Option%201 "/Game/Art/Minigames/Ana/MI_AnaLabyrinth_Button_01_Pressed.MI_AnaLabyrinth_Button_01_Pressed" :Option%202 "/Game/Art/Minigames/Ana/MI_AnaLabyrinth_Button_02_Pressed.MI_AnaLabyrinth_Button_02_Pressed" :Option%203 "/Game/Art/Minigames/Ana/MI_AnaLabyrinth_Button_03_Pressed.MI_AnaLabyrinth_Button_03_Pressed" :Option%204 "/Game/Art/Minigames/Ana/MI_AnaLabyrinth_Button_04_Pressed.MI_AnaLabyrinth_Button_04_Pressed") (Utilities|Select :Index (Variables|Default|GetgateIndex) :Option%200 "/Game/Art/Minigames/Ana/MI_AnaLabyrinth_Button_04_Unpressed.MI_AnaLabyrinth_Button_04_Unpressed" :Option%201 "/Game/Art/Minigames/Ana/MI_AnaLabyrinth_Button_01_Unpressed.MI_AnaLabyrinth_Button_01_Unpressed" :Option%202 "/Game/Art/Minigames/Ana/MI_AnaLabyrinth_Button_02_Unpressed.MI_AnaLabyrinth_Button_02_Unpressed" :Option%203 "/Game/Art/Minigames/Ana/MI_AnaLabyrinth_Button_03_Unpressed.MI_AnaLabyrinth_Button_03_Unpressed" :Option%204 "/Game/Art/Minigames/Ana/MI_AnaLabyrinth_Button_04_Unpressed.MI_AnaLabyrinth_Button_04_Unpressed")))
  (bind _asbp_player_controller (Utilities|Casting|CastToBP_playerController (Game|GetPlayerController 0)))
  (if _isa
    (Default|AnaButtonon (Variables|/Game/Blueprints/Core/BP_playerController.BP_playerController_C|GetsoundControllerRef _asbp_player_controller))
    (else
      (Default|AnaButtonOff (Variables|/Game/Blueprints/Core/BP_playerController.BP_playerController_C|GetsoundControllerRef _asbp_player_controller)))))

(fn ConstructionScript
  (|CallParentFunction)
  (Components|StaticMesh|SetStaticMesh (Variables|Default|Getbutton) (Utilities|Select :Index (Variables|Default|GetgateIndex) :Option%200 "/Game/Art/Minigames/Ana/SM_AnaLabyrinth_Button_04.SM_AnaLabyrinth_Button_04" :Option%201 "/Game/Art/Minigames/Ana/SM_AnaLabyrinth_Button_01.SM_AnaLabyrinth_Button_01" :Option%202 "/Game/Art/Minigames/Ana/SM_AnaLabyrinth_Button_02.SM_AnaLabyrinth_Button_02" :Option%203 "/Game/Art/Minigames/Ana/SM_AnaLabyrinth_Button_03.SM_AnaLabyrinth_Button_03" :Option%204 "/Game/Art/Minigames/Ana/SM_AnaLabyrinth_Button_04.SM_AnaLabyrinth_Button_04"))
  (Rendering|Material|SetMaterial (Variables|Default|Getbutton) 0 (Utilities|Select :Index (Variables|Default|GetgateIndex) :Option%200 "/Game/Art/Minigames/Ana/MI_AnaLabyrinth_Button_04_Unpressed.MI_AnaLabyrinth_Button_04_Unpressed" :Option%201 "/Game/Art/Minigames/Ana/MI_AnaLabyrinth_Button_01_Unpressed.MI_AnaLabyrinth_Button_01_Unpressed" :Option%202 "/Game/Art/Minigames/Ana/MI_AnaLabyrinth_Button_02_Unpressed.MI_AnaLabyrinth_Button_02_Unpressed" :Option%203 "/Game/Art/Minigames/Ana/MI_AnaLabyrinth_Button_03_Unpressed.MI_AnaLabyrinth_Button_03_Unpressed" :Option%204 "/Game/Art/Minigames/Ana/MI_AnaLabyrinth_Button_04_Unpressed.MI_AnaLabyrinth_Button_04_Unpressed")))