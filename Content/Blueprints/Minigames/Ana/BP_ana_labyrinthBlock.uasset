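; Grid block for Ana's labyrinth minigame that acts as either wall or non-wall, set by the IsWall flag.
; The construction script colors the cube black for walls and gray otherwise.
; Shortly after BeginPlay, the box's response to a custom collision channel (GameTraceChannel2) is set to Overlap for walls and Ignore for other blocks.
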(event Custom|prepareCollisions
  ;[1 0.4264 0 0.5] prepareCollisions
  (Utilities|FlowControl|Delay 0.01)
  (Collision|SetCollisionResponsetoChannel (Variables|Default|GetBox) "ECC_GameTraceChannel2" (select (Variables|Default|GetisWall) "ECR_Overlap" "ECR_Ignore")))

(event EventBeginPlay
  ;[1 0.3029 0 0.5] beginPlay
  (CallFunction|PrepareCollisions))

(fn ConstructionScript
  (Rendering|Material|SetMaterial (Variables|Default|GetCube) 0 (select (Variables|Default|GetisWall) "/Game/Testing/materials/solidColorMats/M_testingSolidColorBlack.M_testingSolidColorBlack" "/Game/Testing/materials/solidColorMats/M_testingSolidColorGray.M_testingSolidColorGray")))