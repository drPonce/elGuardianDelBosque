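; Torch (lantern) actor for Ana's minigame, with a drifting light and a one-way "used" sequence.
; On BeginPlay a self-restarting timeline slides Light back along its local X axis, snapping to the start each loop.
; torchUsed makes Box ignore a custom collision channel, then after a short delay shrinks Farol, collapses Light and hides both.
; The construction script gives Cube a gray test material.
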(event Custom|torchUsed
  ;[0.1042 0.1042 0.1042 0.5] torch used
  (Collision|SetCollisionResponsetoChannel (Variables|Default|GetBox) "ECC_GameTraceChannel2" "ECR_Ignore")
  (Utilities|FlowControl|Delay 1.0)
  (Components|Timeline|SetPlayRate (Variables|Default|GetTimeline_0) 0.4)
  (bind _newtrack_1 (Timeline|Timeline_0 PlayFromStart)
    (:Update
      (Transformation|SetRelativeScale3D (Variables|Default|Getfarol) (Math|Vector|Lerp(Vector) "1.200000,1.200000,1.200000" "0, 0, 0" _newtrack_1))
      (Transformation|SetRelativeScale3D (Variables|Default|GetLight) "0, 0, 0"))
    (:Finished
      (Rendering|SetVisibility (Variables|Default|Getfarol) false false))))

(event Custom|lightFloatee
  (bind _light (Variables|Default|GetLight))
  (bind _relativelocation (Variables|/Script/Engine.SceneComponent|GetRelativeLocation _light))
  ;[1 0.4873 0.5131 0.5] light floatee
  (Utilities|FlowControl|Sequence
    (:then_0
      (Components|Timeline|SetPlayRate (Variables|Default|GetTimeline) 0.3)
      (bind _newtrack_0 (Timeline|Timeline PlayFromStart)
        (:Update
          (Transformation|SetRelativeLocation (Variables|Default|GetLight) (Math|Vector|MakeVector (Math|Float|Lerp 25.0 -25.0 _newtrack_0) (.y _relativelocation) (.z _relativelocation)) false false))
        (:Finished
          (Timeline|Timeline PlayFromStart))))))

(event EventBeginPlay
  ;[1 0.3307 0 0.5] begin play
  (|CallParentFunction)
  (CallFunction|LightFloatee))

(fn ConstructionScript
  (|CallParentFunction)
  (Rendering|Material|SetMaterial (Variables|Default|GetCube) 0 "/Game/Testing/materials/solidColorMats/M_testingSolidColorGray.M_testingSolidColorGray"))