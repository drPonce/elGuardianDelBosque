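; Player pawn for Ana's labyrinth minigame, stepping through a grid in fog of war.
; Four directional spheres block moves and detect interactables; timelines drive steps, which repeat while held, and mesh turning.
; Torches raise the light level, widening fog circle and ortho camera; buttons toggle matching gates, while light gates and the exit trigger require level three.
; BeginPlay also calls WinMinigame after four seconds, regardless of progress.
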(event OnComponentBeginOverlap(Sphere_up)
  (params (OverlappedComponent :type Primitive%20Component%20Object%20Reference) (OtherActor :type Actor%20Object%20Reference) (OtherComp :type Primitive%20Component%20Object%20Reference) (OtherBodyIndex :type Integer) (bFromSweep :type Boolean) (SweepResult :type Hit%20Result%20Structure%20%28by%20ref%29))
  ;[0.4518 0.5521 0 0.5] begin overlap
  (Variables|Default|SetupColliding true)
  (Utilities|CheckifNearInteractables OtherActor))

(event OnComponentBeginOverlap(Sphere_down)
  (params (OverlappedComponent :type Primitive%20Component%20Object%20Reference) (OtherActor :type Actor%20Object%20Reference) (OtherComp :type Primitive%20Component%20Object%20Reference) (OtherBodyIndex :type Integer) (bFromSweep :type Boolean) (SweepResult :type Hit%20Result%20Structure%20%28by%20ref%29))
  ;[0.4518 0.5521 0 0.5] begin overlap
  (Variables|Default|SetdownColliding true)
  (Utilities|CheckifNearInteractables OtherActor))

(event OnComponentEndOverlap(Sphere_down)
  (params (OverlappedComponent :type Primitive%20Component%20Object%20Reference) (OtherActor :type Actor%20Object%20Reference) (OtherComp :type Primitive%20Component%20Object%20Reference) (OtherBodyIndex :type Integer))
  ;[0.4518 0.5521 0 0.5] end overlap
  (Variables|Default|SetdownColliding false)
  (CallFunction|EnableDisableHUDButton false OtherActor))

(event OnComponentEndOverlap(Sphere_up)
  (params (OverlappedComponent :type Primitive%20Component%20Object%20Reference) (OtherActor :type Actor%20Object%20Reference) (OtherComp :type Primitive%20Component%20Object%20Reference) (OtherBodyIndex :type Integer))
  ;[0.4518 0.5521 0 0.5] end overlap
  (Variables|Default|SetupColliding false)
  (CallFunction|EnableDisableHUDButton false OtherActor))

(event OnComponentBeginOverlap(Sphere_left)
  (params (OverlappedComponent :type Primitive%20Component%20Object%20Reference) (OtherActor :type Actor%20Object%20Reference) (OtherComp :type Primitive%20Component%20Object%20Reference) (OtherBodyIndex :type Integer) (bFromSweep :type Boolean) (SweepResult :type Hit%20Result%20Structure%20%28by%20ref%29))
  ;[0.4518 0.5521 0 0.5] begin overlap
  (Variables|Default|SetleftColliding true)
  (Utilities|CheckifNearInteractables OtherActor))

(event OnComponentEndOverlap(Sphere_left)
  (params (OverlappedComponent :type Primitive%20Component%20Object%20Reference) (OtherActor :type Actor%20Object%20Reference) (OtherComp :type Primitive%20Component%20Object%20Reference) (OtherBodyIndex :type Integer))
  ;[0.4518 0.5521 0 0.5] end overlap
  (Variables|Default|SetleftColliding false)
  (CallFunction|EnableDisableHUDButton false OtherActor))

(event OnComponentBeginOverlap(Sphere_right)
  (params (OverlappedComponent :type Primitive%20Component%20Object%20Reference) (OtherActor :type Actor%20Object%20Reference) (OtherComp :type Primitive%20Component%20Object%20Reference) (OtherBodyIndex :type Integer) (bFromSweep :type Boolean) (SweepResult :type Hit%20Result%20Structure%20%28by%20ref%29))
  ;[0.4518 0.5521 0 0.5] begin overlap
  (Variables|Default|SetrightColliding true)
  (Utilities|CheckifNearInteractables OtherActor))

(event OnComponentEndOverlap(Sphere_right)
  (params (OverlappedComponent :type Primitive%20Component%20Object%20Reference) (OtherActor :type Actor%20Object%20Reference) (OtherComp :type Primitive%20Component%20Object%20Reference) (OtherBodyIndex :type Integer))
  ;[0.4518 0.5521 0 0.5] end overlap
  (Variables|Default|SetrightColliding false)
  (CallFunction|EnableDisableHUDButton false OtherActor))

(event Custom|moveToPoint
  (params (direction :type directions%20Enum :default "NewEnumerator0"))
  ;[0.6762 0.8521 1 0.5] move the pawn to the desired location
  (CallFunction|RotateBuboMesh direction)
  (Variables|Default|SetmoveButtonBeingPressed true)
  (if (not (Utilities|Select :Index direction :NewEnumerator0 (Variables|Default|GetupColliding) :NewEnumerator1 (Variables|Default|GetdownColliding) :NewEnumerator2 (Variables|Default|GetleftColliding) :NewEnumerator3 (Variables|Default|GetrightColliding))) ; queremos que no haya un\nmuro en la direccion que\nnos estamos intentando mover\npara movernos
    (if (not (Variables|Default|GetcurrentlyMoving)) ; if we are moving we must\nwait until we can move again
      (Variables|Default|SetcurrentMovingDirection direction)
      (Collision|SetCollisionResponsetoChannel (Variables|Default|GetSphere_up) "ECC_GameTraceChannel1" "ECR_Ignore") ; deactivateCollisions
      (Utilities|FlowControl|Sequence
        (:then_0
          (Variables|Default|SetcurrentlyMoving true))
        (:then_1
          (Variables|Default|SetinteractWithButtonPossible false))
        (:then_2
          (Variables|Default|SetinteractWithTorchPossible false))
        (:then_3
          (Variables|Default|SetlocationBeforeMoving (Transformation|GetActorLocation))
          (Components|Timeline|SetPlayRate (Variables|Default|GetmoveAnimation) 3.0)
          (bind _delta (Timeline|moveAnimation PlayFromStart)
            (:Update
              (Transformation|SetActorLocation (Math|Vector|Lerp(Vector) (Variables|Default|GetlocationBeforeMoving) (+ (Variables|Default|GetlocationBeforeMoving) (Utilities|Select :Index (Variables|Default|GetcurrentMovingDirection) :NewEnumerator0 "-200.000000,0.000000,0.000000" :NewEnumerator1 "200.000000,0.000000,0.000000" :NewEnumerator2 "0.000000,200.000000,0.000000" :NewEnumerator3 "0.000000,-200.000000,0.000000")) _delta) false false))
            (:Finished
              (CallFunction|AfterMoveActions))))))))

(event Custom|moveButtonReleased
  ;[0.6762 0.8521 1 0.5] move the pawn to the desired location
  ;;[0.6193 0.8682 1 0.5] when any move button releases
  (Variables|Default|SetmoveButtonBeingPressed false))

(event Custom|afterMoveActions
  ;[0.6013 0.7871 1 0.5] actions after the move animation ends. keep the loop on if the button is still pressed
  ;;[0.5323 0.7504 1 0.5] set the collisions and the boolean as im still again
  (Variables|Default|SetcurrentlyMoving false)
  (Collision|SetCollisionResponsetoChannel (Variables|Default|GetSphere_up) "ECC_GameTraceChannel1" "ECR_Overlap") ; activateCollisions
  (Utilities|FlowControl|Delay 0.001) ; tiempo supersticioso
  (if (Variables|Default|GetmoveButtonBeingPressed) ; is the mouse buttonStillBeing\nPressed?
    (CallFunction|MovetoPoint (Variables|Default|GetcurrentPressedButton))))

(event Custom|interactButtonPressed
  ;[1 0 0.7381 0.5] interact button pressed
  (if (Variables|Default|GetinteractWithTorchPossible)
    (CallFunction|AugmentLight)
    (elif (Variables|Default|GetinteractWithLightGatePossible)
      (bind _outactors (Actor|GetAllActorsOfClass "/Game/Blueprints/Minigames/Ana/BP_ana_lightGate.BP_ana_lightGate_C"))
      (for _array_element _outactors
        (Default|SwitchOpenClose _array_element))
      (elif (Variables|Default|GetinteractWithButtonPossible)
        (Utilities|FlowControl|Sequence
          (:then_0
            (bind _outactors_2 (Actor|GetAllActorsOfClass "/Game/Blueprints/Minigames/Ana/BP_ana_gate.BP_ana_gate_C"))
            (for _array_element_2 _outactors_2
              (if (== (Variables|/Game/Blueprints/Minigames/Ana/BP_ana_gate.BP_ana_gate_C|GetgateIndex _array_element_2) (Variables|Default|GetnearButtonGateIndex))
                (Default|SwitchOpenClose _array_element_2))))
          (:then_1
            (bind _outactors_3 (Actor|GetAllActorsOfClass "/Game/Blueprints/Minigames/Ana/BP_ana_button.BP_ana_button_C"))
            (for _array_element_3 _outactors_3
              (if (== (Variables|/Game/Blueprints/Minigames/Ana/BP_ana_button.BP_ana_button_C|GetgateIndex _array_element_3) (Variables|Default|GetnearButtonGateIndex))
                (Default|SwitchBetweenPressedandUnpressed _array_element_3)))))))))

(event Custom|augmentLight
  (bind _currentlightlevel (Variables|Default|GetcurrentLightLevel))
  (bind _currentlightlevel_2 (Variables|Default|GetcurrentLightLevel))
  ;[0.6097 0.3476 1 0.5] augment light
  (Default|TorchUsed (Variables|Components|GetnearTorchReference))
  (Math|Integer|IncrementInt _currentlightlevel_2
    (:%20%20
      (Variables|Default|SetinteractWithTorchPossible false) ; para que no se pueda repetir
      (bind _newtrack_1 (Timeline|Timeline_0 PlayFromStart)
        (:Update
          (Rendering|Material|SetScalarParameterValue (Variables|Components|GetvignetteMaterialReference) "circleSize" (Math|Float|Lerp (Utilities|Select :Index (- (Variables|Default|GetcurrentLightLevel) 1) :Option%200 (Variables|Default|GetcirclePetiteness_light0) :Option%201 (Variables|Default|GetcirclePetiteness_light1) :Option%202 (Variables|Default|GetcirclePetiteness_light2) :Option%203 (Variables|Default|GetcirclePetiteness_light3)) (Utilities|Select :Index _currentlightlevel_2 :Option%200 (Variables|Default|GetcirclePetiteness_light0) :Option%201 (Variables|Default|GetcirclePetiteness_light1) :Option%202 (Variables|Default|GetcirclePetiteness_light2) :Option%203 (Variables|Default|GetcirclePetiteness_light3)) _newtrack_1) :!class /Script/Engine.MaterialInstanceDynamic))
        (:Finished
          (Utilities|FlowControl|Sequence
            (:then_0
              (bind _outactors (Actor|GetAllActorsOfClass "/Game/Blueprints/Minigames/Ana/BP_ana_lightGate.BP_ana_lightGate_C"))
              (for _array_element _outactors
                (Default|ReceiveLight _array_element)))
            (:then_1
              ;;[1 0.7477 0 0.5] HEAH
              (Utilities|FlowControl|Delay 1.0)
              (bind _newtrack_1_2 (Timeline|Timeline_1 PlayFromStart)
                (:Update
                  (Class|CameraComponent|SetOrthoWidth (Variables|Default|GetCamera) (Math|Float|Lerp (Utilities|Select :Index (- _currentlightlevel 1) :Option%200 (Variables|Default|GetorthoWidth_light0) :Option%201 (Variables|Default|GetorthoWidth_light1) :Option%202 (Variables|Default|GetorthoWidth_light2) :Option%203 (Variables|Default|GetorthoWidth_light3)) (Utilities|Select :Index _currentlightlevel :Option%200 (Variables|Default|GetorthoWidth_light0) :Option%201 (Variables|Default|GetorthoWidth_light1) :Option%202 (Variables|Default|GetorthoWidth_light2) :Option%203 (Variables|Default|GetorthoWidth_light3)) _newtrack_1_2)))))))))))

(event Custom|MovePlayerToStartLocation
  (params (DifficultyIndex :type Integer))
  ;[0.3698 0.143 0 0.5] Move Player to StartLocation
  (Transformation|SetActorLocation (Utilities|Select :Index DifficultyIndex :Option%200 "0, 0, 0" :Option%201 (Variables|Default|GetStartLocationLvl1) :Option%202 (Variables|Default|GetStartLocationLvl2) :Option%203 (Variables|Default|GetStartLocationLvl3)) false false))

(event Custom|rotateBuboMesh
  (params (direction :type directions%20Enum :default "NewEnumerator0"))
  ;[0.6026 0.4549 1 0.5] spin bubo
  (bind _newtrack_0 (Timeline|Timeline PlayFromStart)
    (:Update
      (Transformation|SetRelativeRotation (Variables|Default|GetbuboMesh) (Math|Rotator|MakeRotator 0.0 0.0 (- (Math|Float|Lerp (Utilities|Select :Index (Variables|Default|GetlastDirectionLooked) :NewEnumerator0 -9e+01 :NewEnumerator1 9e+01 :NewEnumerator2 1.8e+02 :NewEnumerator3 0.0) (Utilities|Select :Index (Variables|Default|GetlastDirectionLooked) :NewEnumerator0 (Utilities|Select :Index direction :NewEnumerator0 -9e+01 :NewEnumerator1 9e+01 :NewEnumerator2 -1.8e+02 :NewEnumerator3 0.0) :NewEnumerator1 (Utilities|Select :Index direction :NewEnumerator0 -9e+01 :NewEnumerator1 9e+01 :NewEnumerator2 1.8e+02 :NewEnumerator3 0.0) :NewEnumerator2 (Utilities|Select :Index direction :NewEnumerator0 2.7e+02 :NewEnumerator1 9e+01 :NewEnumerator2 1.8e+02 :NewEnumerator3 0.0) :NewEnumerator3 (Utilities|Select :Index direction :NewEnumerator0 -9e+01 :NewEnumerator1 9e+01 :NewEnumerator2 -1.8e+02 :NewEnumerator3 0.0)) _newtrack_0) 9e+01)) false false))
    (:Finished
      (Variables|Default|SetlastDirectionLooked direction))))

(event Custom|enableDisableHUDButton
  (params (trueMeansEnable :type Boolean) (otherActor :type Object%20Object%20Reference))
  ;[1 0.7269 0.835 0.5] enable disable interact button
  (Utilities|Casting|CastToBP_ana_torch otherActor ; solo nos interesa si lo que nos hemos alejado o acercado de\nes un buton o antorcha (las puertas o muros no cuentan)\n\nañadimos ahora la lightgate que solo va a encender el boton\nsi el nivel de luz es el correcto
    (:then
      (bind _asbp_player_controller (Utilities|Casting|CastToBP_playerController (Game|GetPlayerController 0) :!label _label))
      (bind _asui_ana (Utilities|Casting|CastToUI_ana (Variables|/Game/Blueprints/Core/BP_playerController.BP_playerController_C|Getminigame_UI_reference _asbp_player_controller)))
      (Widget|SetIsEnabled (Variables|/Game/Blueprints/Widgets/minigames/ana/UI_ana.UI_ana_C|GetinteractButton _asui_ana) trueMeansEnable))
    (:CastFailed
      (Utilities|Casting|CastToBP_ana_button otherActor
        (:then
          (goto _label))
        (:CastFailed
          (Utilities|Casting|CastToBP_ana_lightGate otherActor)
          (if (>= (Variables|Default|GetcurrentLightLevel) 3)
            (goto _label)))))))

(event EventBeginPlay
  ;[1 0.5486 0 0.5] begin the player playing play
  (Utilities|FlowControl|Sequence
    (:then_0
      (Class|CameraComponent|SetOrthoWidth (Variables|Default|GetCamera) (Variables|Default|GetorthoWidth_light0)) ; new for pauli
      (Utilities|FlowControl|Delay 4.0)
      (bind _asbp_player_controller (Utilities|Casting|CastToBP_playerController (Game|GetPlayerController 0)))
      (Default|WinMinigame _asbp_player_controller))
    (:then_1
      ;;[1 0.4105 0 0.5] prepare collisions at the begin play
      (Utilities|FlowControl|Delay 0.1)
      (Collision|SetCollisionResponsetoChannel (Variables|Default|GetSphere_up) "ECC_GameTraceChannel1" "ECR_Overlap"))))

(fn ConstructionScript
  (bind _returnvalue (Rendering|Material|CreateDynamicMaterialInstance (Variables|Default|GetPlane) 0 "/Game/Art/Minigames/Ana/M_AnaLabyrinth_FogofWar.M_AnaLabyrinth_FogofWar" "None" :!class /Script/Engine.PrimitiveComponent))
  (bind _output_get (Variables|Components|SetvignetteMaterialReference _returnvalue))
  (Rendering|Material|SetScalarParameterValue _output_get "circleSize" (Variables|Default|GetcirclePetiteness_light0) :!class /Script/Engine.MaterialInstanceDynamic))