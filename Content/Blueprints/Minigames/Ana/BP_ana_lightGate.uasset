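; Double-door light gate for Ana's labyrinth minigame, oriented horizontally or vertically by the construction script.
; Toggling or initializing its closed state sets whether the box overlaps or ignores a custom trace channel, then plays the open/close animation.
; Staggered timelines swing both gate meshes and fade the lanterns' shared dynamic material through "Block Opacity".
; Each received light reveals the next of three light-level meshes through a non-looping MultiGate.
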(event Custom|switchOpenClose
  ;[1 0.4411 0.7244 0.5] switchOpenClose
  (Variables|Default|SetisClosed (not (Variables|Default|GetisClosed))) ; switch its previous value
  ;;[1 0.4411 0.7244 0.5] set collision depending on open or closed
  (Collision|SetCollisionResponsetoChannel (Variables|Default|GetBox) "ECC_GameTraceChannel2" (select (Variables|Default|GetisClosed) "ECR_Overlap" "ECR_Ignore"))
  (Utilities|FlowControl|Delay 0.2)
  (CallFunction|OpenCloseGateAnimation (not (Variables|Default|GetisClosed))))

(event Custom|receiveLight
  ;[1 0 0.5977 0.5] receive light
  (Utilities|FlowControl|MultiGate false false -1
    (:Out%200
      (Rendering|SetVisibility (Variables|Default|GetlightLevel1) true false))
    (:Out%201
      (Rendering|SetVisibility (Variables|Default|GetlightLevel2) true false))
    (:Out%202
      (Rendering|SetVisibility (Variables|Default|GetlightLevel3) true false))))

(event Custom|openCloseGateAnimation
  (params (trueMeansOpen :type Boolean))
  ;[0.51 1 0.5255 0.5] open lock animation
  (Utilities|FlowControl|Sequence
    (:then_0
      (Utilities|FlowControl|Delay (select trueMeansOpen 0.0 0.4))
      (Components|Timeline|SetPlayRate (Variables|Default|GetgateOpen) 1.0)
      (if trueMeansOpen
        (bind _newtrack_0 (Timeline|Timeline PlayFromStart)
          (:Update
            (Rendering|Material|SetScalarParameterValue (Variables|Default|GetlightMaterial) "Block Opacity" _newtrack_0 :!class /Script/Engine.MaterialInstanceDynamic)))
        (else
          (Timeline|Timeline ReverseFromEnd))))
    (:then_1
      (Utilities|FlowControl|Delay (select trueMeansOpen 1.2 0.0))
      (Components|Timeline|SetPlayRate (Variables|Default|GetgateOpen) 1.5)
      (if trueMeansOpen
        (bind _newtrack_0_2 (Timeline|gateOpen PlayFromStart)
          (:Update
            (Transformation|SetRelativeRotation (Variables|Default|GetgateMesh) (Math|Rotator|MakeRotator 0.0 0.0 (Math|Float|Lerp 1.8e+02 2.7e+02 _newtrack_0_2)) false false)
            (Transformation|SetRelativeRotation (Variables|Default|GetgateMesh1) (Math|Rotator|MakeRotator 0.0 0.0 (Math|Float|Lerp 0.0 -9e+01 _newtrack_0_2)) false false)))
        (else
          (Timeline|gateOpen ReverseFromEnd))))))

(event Custom|beginPlayOpenClose
  ;[1 0.4411 0.7244 0.5] switchOpenClose
  ;;[1 0.4411 0.7244 0.5] set collision depending on open or closed
  (Collision|SetCollisionResponsetoChannel (Variables|Default|GetBox) "ECC_GameTraceChannel2" (select (Variables|Default|GetisClosed) "ECR_Overlap" "ECR_Ignore"))
  (Utilities|FlowControl|Delay 0.2)
  (CallFunction|OpenCloseGateAnimation (not (Variables|Default|GetisClosed))))

(event EventPrepareCollisions
  ;[1 0.4719 0 0.5] prepareCollisionsOverride
  ;;[1 0.3842 0.002751 0.5] set collision depending on open or closed
  (Collision|SetCollisionResponsetoChannel (Variables|Default|GetBox) "ECC_GameTraceChannel2" (select (Variables|Default|GetisClosed) "ECR_Overlap" "ECR_Ignore"))
  (CallFunction|BeginPlayOpenClose))

(fn ConstructionScript
  (|CallParentFunction)
  ;[1 1 1 0.5] rotate the gate root depending on the boolean
  (Transformation|SetRelativeRotation (Variables|Default|GetgateRoot) (select (Variables|Default|GetisHorizontal) "0, 0, 0" "0.000000,90.000000,0.000000") false false)
  (bind _returnvalue (Rendering|Material|CreateDynamicMaterialInstance (Variables|Default|GetlightLevel1) 0 "/Game/Art/Minigames/Ana/MI_AnaLabyrinth_Larntern_Light.MI_AnaLabyrinth_Larntern_Light" "None" :!class /Script/Engine.PrimitiveComponent))
  (bind _output_get (Variables|Default|SetlightMaterial _returnvalue))
  (Rendering|Material|SetMaterial (Variables|Default|GetlightLevel2) 0 _output_get))