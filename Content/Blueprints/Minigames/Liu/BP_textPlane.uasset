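; BP_textPlane is a minigame plane that reveals up to three lines of text one at a time through material opacity.
; The construction script creates a dynamic material from CustomMaterial.
; Each increment advances the index and, after a short delay, plays a timeline fading in that line's opacity parameter; rewind zeroes all three.
; When the index reaches MaxTextIndex, it waits, then calls WinMinigame on the player controller.
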(event Custom|incrementText
  ;[0 0.6928 1 0.5] increment text
  (Math|Integer|IncrementInt (Variables|Default|GetcurrentTextIndex)
    (:%20%20
      (Utilities|FlowControl|Delay 0.2)
      (bind _newtrack_0 (Timeline|fadeText PlayFromStart)
        (:Update
          (Rendering|Material|SetScalarParameterValue (Variables|Default|GetdynamicMaterialRef) (Utilities|Select :Index (Variables|Default|GetcurrentTextIndex) :Option%200 "ggo" :Option%201 "Line 01 Opacity" :Option%202 "Line 02 Opacity" :Option%203 "Line 03 Opacity") _newtrack_0 :!class /Script/Engine.MaterialInstanceDynamic))
        (:Finished
          (if (>= (Variables|Default|GetcurrentTextIndex) (Variables|Default|GetmaxTextIndex))
            (Utilities|FlowControl|Delay 1.0)
            (bind _asbp_player_controller (Utilities|Casting|CastToBP_playerController (Game|GetPlayerController 0)))
            (Default|WinMinigame _asbp_player_controller)))))))

(event Custom|rewindText
  ;[1 0.7179 0.6144 0.5] rewindBack
  (Variables|Default|SetcurrentTextIndex 0)
  (for _index (range 1 3)
    (Rendering|Material|SetScalarParameterValue (Variables|Default|GetdynamicMaterialRef) (Utilities|Select :Index _index :Option%200 "ggo" :Option%201 "Line 01 Opacity" :Option%202 "Line 02 Opacity" :Option%203 "Line 03 Opacity") 0.0 :!class /Script/Engine.MaterialInstanceDynamic)))

(fn ConstructionScript
  (bind _returnvalue (Rendering|Material|CreateDynamicMaterialInstance (Variables|Default|GetPlane) 0 (Variables|Default|GetcustomMaterial) "None" :!class /Script/Engine.PrimitiveComponent))
  (Variables|Default|SetdynamicMaterialRef _returnvalue))