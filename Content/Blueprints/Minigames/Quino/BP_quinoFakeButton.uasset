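; Decorative button for the Quino football minigame that gives visual and audio press feedback without triggering any gameplay logic of its own.
; ButtonIndex selects the mesh in the construction script and the matching normal and clicked materials at runtime.
; The miniclick event swaps to the clicked material, plays a UI press sound through the player controller's SoundControllerRef, then restores the normal material after a brief delay.
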(event Custom|miniclick
  (bind _staticmeshcomponent (Variables|Debug|GetStaticMeshComponent))
  (Rendering|Material|SetMaterial _staticmeshcomponent 0 (Utilities|Select :Index (Variables|Default|GetbuttonIndex) :Option%200 "/Game/Art/Minigames/Quino/MI_QuinoFootball_Button_01_clicked.MI_QuinoFootball_Button_01_clicked" :Option%201 "/Game/Art/Minigames/Quino/MI_QuinoFootball_Button_01_clicked.MI_QuinoFootball_Button_01_clicked" :Option%202 "/Game/Art/Minigames/Quino/MI_QuinoFootball_Button_02_clicked.MI_QuinoFootball_Button_02_clicked" :Option%203 "/Game/Art/Minigames/Quino/MI_QuinoFootball_Button_03_clicked.MI_QuinoFootball_Button_03_clicked" :Option%204 "/Game/Art/Minigames/Quino/MI_QuinoFootball_Button_04_clicked.MI_QuinoFootball_Button_04_clicked"))
  (Default|GenericUiPress (Variables|/Game/Blueprints/Core/BP_playerController.BP_playerController_C|GetsoundControllerRef (Variables|Default|GetAs%20BP%20Player%20Controller)) true)
  (Utilities|FlowControl|Delay 0.07)
  (Rendering|Material|SetMaterial _staticmeshcomponent 0 (Utilities|Select :Index (Variables|Default|GetbuttonIndex) :Option%200 "/Game/Art/Minigames/Quino/MI_QuinoFootball_Button_01.MI_QuinoFootball_Button_01" :Option%201 "/Game/Art/Minigames/Quino/MI_QuinoFootball_Button_01.MI_QuinoFootball_Button_01" :Option%202 "/Game/Art/Minigames/Quino/MI_QuinoFootball_Button_02.MI_QuinoFootball_Button_02" :Option%203 "/Game/Art/Minigames/Quino/MI_QuinoFootball_Button_03.MI_QuinoFootball_Button_03" :Option%204 "/Game/Art/Minigames/Quino/MI_QuinoFootball_Button_04.MI_QuinoFootball_Button_04")))

(event EventBeginPlay
  (bind _asbp_player_controller (Utilities|Casting|CastToBP_playerController (Game|GetPlayerController 0)))
  (Variables|Default|SetAs%20BP%20Player%20Controller _asbp_player_controller))

(fn ConstructionScript
  (Components|StaticMesh|SetStaticMesh (Variables|Debug|GetStaticMeshComponent) (Utilities|Select :Index (Variables|Default|GetbuttonIndex) :Option%200 "/Game/Art/Minigames/Quino/SM_button_01.SM_button_01" :Option%201 "/Game/Art/Minigames/Quino/SM_button_01.SM_button_01" :Option%202 "/Game/Art/Minigames/Quino/SM_button_02.SM_button_02" :Option%203 "/Game/Art/Minigames/Quino/SM_button_03.SM_button_03" :Option%204 "/Game/Art/Minigames/Quino/SM_button_04.SM_button_04")))