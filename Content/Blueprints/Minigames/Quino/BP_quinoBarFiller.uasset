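; Quino minigame bar actor that shows Quino's courage points as a progress bar on a mesh material.
; The construction script creates a dynamic instance of the soccer progress bar material.
; Shortly after begin play, and on each moveBarProgress call, it sets the "Mateo Pain" parameter to the current-to-max courage ratio from BP_playerController, clamped so a sliver stays visible.
; Each update also asks the controller to try changing the pain face.
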(event Custom|moveBarProgress
  ;[1 1 1 0.5] move the pain bar progress
  (Rendering|Material|SetScalarParameterValue (Variables|Default|GetbarMatInstance) "Mateo Pain" (Math|Float|Clamp(Float) (/ (Math|Conversions|ToFloat(Integer) (Variables|/Game/Blueprints/Core/BP_playerController.BP_playerController_C|GetquinoCouragePoints (Variables|Default|GetplayConRef))) (Math|Conversions|ToFloat(Integer) (Variables|/Game/Blueprints/Core/BP_playerController.BP_playerController_C|GetquinoMaxCouragePoints (Variables|Default|GetplayConRef)))) 0.05) :!class /Script/Engine.MaterialInstanceDynamic)
  (Default|QuinoTrytoChangePainFace (Variables|Default|GetplayConRef)))

(event EventBeginPlay
  ;[1 0.3528 0 0.5] begin play
  (bind _asbp_player_controller (Utilities|Casting|CastToBP_playerController (Game|GetPlayerController 0)))
  (Variables|Default|SetplayConRef _asbp_player_controller)
  (Utilities|FlowControl|Delay 0.2) ; dale tiempo a que se ponga\nxulo todo
  (CallFunction|MoveBarProgress))

(fn ConstructionScript
  (bind _returnvalue (Rendering|Material|CreateDynamicMaterialInstance (Variables|Debug|GetStaticMeshComponent) 0 "/Game/Art/Minigames/Quino/MI_QuinoSoccer_ProgressBar.MI_QuinoSoccer_ProgressBar" "None" :!class /Script/Engine.PrimitiveComponent))
  (Variables|Default|SetbarMatInstance _returnvalue))