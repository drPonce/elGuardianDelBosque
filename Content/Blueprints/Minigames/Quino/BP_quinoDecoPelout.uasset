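; Decorative "pelout" actor for the Quino minigame, with a master variant that starts visible while the others start transparent.
; The construction script creates a dynamic ball material at zero "Block Opacity", which BeginPlay raises to full for the master.
; A reveal event plays a reversed timeline, copied from the stars, to animate opacity and scale relative to the starting scale.
; A separate master event briefly hides the mesh, then shows it again.
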(event Custom|otherPeloutsMiniReveal
  (bind _scaleonbegin (Variables|Default|GetscaleOnBegin))
  (Components|Timeline|SetPlayRate (Variables|Default|GetTimeline) 0.9)
  (bind (_direction _newtrack_0 _newtrack_1) (Timeline|Timeline PlayFromStart)
    (:Update
      (Rendering|Material|SetScalarParameterValue (Variables|Default|GetmaterialInstance) "Block Opacity" (Math|Float|Lerp 1.0 0.0 _newtrack_0) :!class /Script/Engine.MaterialInstanceDynamic)
      (Transformation|SetActorScale3D (Math|Vector|Lerp(Vector) _scaleonbegin (* _scaleonbegin "0.800000,0.800000,0.800000") _newtrack_1)))))

(event Custom|masterPeloutMiniHide
  (bind _staticmeshcomponent (Variables|Debug|GetStaticMeshComponent))
  (Rendering|SetVisibility _staticmeshcomponent false false)
  (Utilities|FlowControl|Delay 0.2)
  (Rendering|SetVisibility _staticmeshcomponent true false))

(event EventBeginPlay
  (Utilities|FlowControl|Sequence
    (:then_0
      (if (Variables|Default|GetiAmMasterPelout)
        (Rendering|Material|SetScalarParameterValue (Variables|Default|GetmaterialInstance) "Block Opacity" 1.0 :!class /Script/Engine.MaterialInstanceDynamic)))
    (:then_1
      (Variables|Default|SetscaleOnBegin (Transformation|GetActorScale3D)))))

(fn ConstructionScript
  (bind _returnvalue (Rendering|Material|CreateDynamicMaterialInstance (Variables|Debug|GetStaticMeshComponent) 0 "/Game/Art/Minigames/Quino/M_BallSupremacee.M_BallSupremacee" "None" :!class /Script/Engine.PrimitiveComponent))
  (bind _output_get (Variables|Default|SetmaterialInstance _returnvalue))
  (Rendering|Material|SetScalarParameterValue _output_get "Block Opacity" 0.0 :!class /Script/Engine.MaterialInstanceDynamic))