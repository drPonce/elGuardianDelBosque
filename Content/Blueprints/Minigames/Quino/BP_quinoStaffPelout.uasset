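; Beat-note ball for the Quino minigame staff, sliding toward the perfect-beat indicator.
; The construction script picks a mesh by ball color and creates a dynamic material starting at zero opacity.
; It fades in on spawn; Tick then lerps its Y from spawn to beat point using lifetime over the player controller's staff time length.
; Fade-out reverses the opacity timeline and destroys the actor shortly after finishing.
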(event Custom|fadeInOut
  (params (trueMeansFadeIn :type Boolean))
  (if trueMeansFadeIn
    (bind _newtrack_0 (Timeline|Timeline PlayFromStart)
      (:Update
        (Rendering|Material|SetScalarParameterValue (Variables|Components|GetmaterialInstance) "Block Opacity" _newtrack_0 :!class /Script/Engine.MaterialInstanceDynamic))
      (:Finished
        (if (not trueMeansFadeIn) ; si nos fadeamos out, cuando\ntermine nos destruimos
          (Utilities|FlowControl|Delay 0.2)
          (Actor|DestroyActor))))
    (else
      (Timeline|Timeline ReverseFromEnd))))

(event EventBeginPlay
  ;[1 0.2414 0 0.5] begin play
  (bind _asbp_player_controller (Utilities|Casting|CastToBP_playerController (Game|GetPlayerController 0)))
  (Variables|Components|SetplayConRef _asbp_player_controller)
  (Variables|Default|SetbirthTime (Utilities|Time|GetGameTimeinSeconds))
  (Variables|Default|SetreadyToMove true) ; ahora esta aqui but maybe we need to\ndo something else in the future before\nwe set it to ready to move
  (Components|Timeline|SetPlayRate (Variables|Default|GetTimeline) 5.0)
  (CallFunction|FadeinOut true))

(event EventTick
  (params (DeltaSeconds :type Float%20%28single-precision%29))
  (bind _returnvalue (Transformation|GetActorLocation))
  (bind _playconref (Variables|Components|GetplayConRef))
  (if (Variables|Default|GetreadyToMove)
    (Transformation|SetActorLocation (Math|Vector|MakeVector (.x _returnvalue) (Math|Float|Lerp (.y (Variables|/Game/Blueprints/Core/BP_playerController.BP_playerController_C|GetquinoBallSpawnLocation _playconref)) (.y (Variables|/Game/Blueprints/Core/BP_playerController.BP_playerController_C|GetquinoBallPerfectBeatLocation _playconref)) (/ (- (Utilities|Time|GetGameTimeinSeconds) (Variables|Default|GetbirthTime)) (Variables|/Game/Blueprints/Core/BP_playerController.BP_playerController_C|GetballStaffTemporalLength (Variables|Components|GetplayConRef)))) (.z _returnvalue)) false false)))

(fn ConstructionScript
  (bind _peloutmesh (Variables|Default|GetpeloutMesh))
  (Components|StaticMesh|SetStaticMesh _peloutmesh (Utilities|Select :Index (Variables|Default|GetballColor) :NewEnumerator0 "/Game/Art/Minigames/Quino/SM_QuinoSoccer_Ball_04.SM_QuinoSoccer_Ball_04" :NewEnumerator1 "/Game/Art/Minigames/Quino/SM_QuinoSoccer_Ball_03.SM_QuinoSoccer_Ball_03" :NewEnumerator2 "/Game/Art/Minigames/Quino/SM_QuinoSoccer_Ball_01.SM_QuinoSoccer_Ball_01" :NewEnumerator3 "/Game/Art/Minigames/Quino/SM_QuinoSoccer_Ball_02.SM_QuinoSoccer_Ball_02"))
  (bind _returnvalue (Rendering|Material|CreateDynamicMaterialInstance _peloutmesh 0 "/Game/Art/Minigames/Quino/MI_QuinoSoccer_GeneralAssets02.MI_QuinoSoccer_GeneralAssets02" "None" :!class /Script/Engine.PrimitiveComponent))
  (bind _output_get (Variables|Components|SetmaterialInstance _returnvalue))
  (Rendering|Material|SetScalarParameterValue _output_get "Block Opacity" 0.0 :!class /Script/Engine.MaterialInstanceDynamic))