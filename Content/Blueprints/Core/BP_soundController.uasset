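; Central sound controller that plays the game's one-shot 2D effects through named events, grouped into graphs for Liu, Ana, Quino and generic UI, minigame and celebration sounds.
; Sound families vary through random looping MultiGates and randomized pitch, and the Ana button events also trigger door-movement sounds.
; A gate-and-delay MiniCooldown macro throttles rewind and UI press sounds.
; The EventGraph holds an empty sound-family template and a debug event cycling Quino's shot sounds.
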(event Custom|soundFamTemp
  ;[1 1 1 0.5] sound family template
  (Utilities|FlowControl|MultiGate true true -1
    (:Out%200
      (Audio|PlaySound2D 0 (Math|Float|MakeLiteralFloat 1.0) (Math|Random|RandomFloatinRange 1.0 1.0) 0.0 0 0))))

(event Custom|debuggingTry
  (Utilities|FlowControl|MultiGate false true -1
    (:Out%200
      (CallFunction|QuinoGudShot))
    (:Out%201
      (CallFunction|QuinoMidShot))
    (:Out%202
      (CallFunction|QuinoBadShot))))

(event Custom|liuPieceWon
  (params (Index :type Integer))
  ;[1 1 1 0.5] Comment
  (Audio|PlaySound2D (Utilities|Select :Index Index :Option%200 "/Game/NotFMOD/source/sfx/minigames/liu/piecewon/liuPieceWon.liuPieceWon" :Option%201 "/Game/NotFMOD/source/sfx/minigames/liu/piecewon/liuPieceWon.liuPieceWon" :Option%202 "/Game/NotFMOD/source/sfx/minigames/liu/piecewon/liuPieceWon2.liuPieceWon2" :Option%203 "/Game/NotFMOD/source/sfx/minigames/liu/piecewon/liuPieceWon3.liuPieceWon3") (Math|Float|MakeLiteralFloat 1.3) 1.0 0.0 0 0))

(event Custom|liu_movePiece
  (bind _returnvalue (Math|Float|MakeLiteralFloat 0.7))
  (bind _returnvalue_2 (Math|Random|RandomFloatinRange 0.6 1.4))
  ;[1 1 1 0.5] alor alor alor
  (Utilities|FlowControl|MultiGate true true -1
    (:Out%200
      (Audio|PlaySound2D "/Game/NotFMOD/source/sfx/minigames/liu/pieceMove/Mover_piezas_5.Mover_piezas_5" _returnvalue _returnvalue_2 0.0 0 0))
    (:Out%201
      (Audio|PlaySound2D "/Game/NotFMOD/source/sfx/minigames/liu/pieceMove/Mover_piezas_8.Mover_piezas_8" _returnvalue _returnvalue_2 0.0 0 0))
    (:Out%202
      (Audio|PlaySound2D "/Game/NotFMOD/source/sfx/minigames/liu/pieceMove/Mover_piezas_6.Mover_piezas_6" _returnvalue _returnvalue_2 0.0 0 0))
    (:Out%203
      (Audio|PlaySound2D "/Game/NotFMOD/source/sfx/minigames/liu/pieceMove/Mover_piezas_9.Mover_piezas_9" _returnvalue _returnvalue_2 0.0 0 0))))

(event Custom|liu_selectPiece
  (bind _returnvalue (Math|Float|MakeLiteralFloat 0.2))
  (bind _returnvalue_2 (Math|Random|RandomFloatinRange 1.2 2.2))
  ;[1 1 1 0.5] alor alor alor
  (Utilities|FlowControl|MultiGate true true -1
    (:Out%200
      (Audio|PlaySound2D "/Game/NotFMOD/source/sfx/minigames/liu/pieceSelect/Seleccionar-pieza-1.Seleccionar-pieza-1" _returnvalue _returnvalue_2 0.0 0 0))
    (:Out%201
      (Audio|PlaySound2D "/Game/NotFMOD/source/sfx/minigames/liu/pieceSelect/Seleccionar-pieza-3.Seleccionar-pieza-3" _returnvalue _returnvalue_2 0.0 0 0))
    (:Out%202
      (Audio|PlaySound2D "/Game/NotFMOD/source/sfx/minigames/liu/pieceSelect/Seleccionar-pieza-5.Seleccionar-pieza-5" _returnvalue _returnvalue_2 0.0 0 0))))

(event Custom|liu_rewind
  ;[1 1 1 0.5] Comment
  (Utilities|MiniCooldown 0.3)
  (Audio|PlaySound2D "/Game/NotFMOD/source/sfx/minigames/liu/returnLiu.returnLiu" (Math|Float|MakeLiteralFloat 1.2) (Math|Random|RandomFloatinRange 0.9 1.3) 0.0 0 0))

(event Custom|generic_pauseButtonPress
  ;[1 1 1 0.5] Comment
  (Audio|PlaySound2D "/Game/NotFMOD/source/sfx/generic/ui/pauseButton.pauseButton" (Math|Float|MakeLiteralFloat 1.2) (Math|Random|RandomFloatinRange 0.8 1.1) 0.0 0 0))

(event Custom|generic_uiPress
  (params (loud :type Boolean))
  ;[1 1 1 0.5] Comment
  (Utilities|MiniCooldown 0.2)
  (Audio|PlaySound2D "/Game/NotFMOD/source/sfx/generic/ui/uiPress.uiPress" (select loud 0.6 0.3) (Math|Float|MakeLiteralFloat 0.8) 0.0 0 0))

(event Custom|generic_fanfare
  ;[1 1 1 0.5] Comment
  (Utilities|FlowControl|Sequence
    (:then_0
      (Audio|PlaySound2D "/Game/NotFMOD/source/sfx/generic/minigamesGeneral/fanfarria.fanfarria" (Math|Float|MakeLiteralFloat 1.0) (Math|Random|RandomFloatinRange 1.0 1.0) 0.0 0 0))))

(event Custom|generic_buboYelling
  (bind _returnvalue (Math|Float|MakeLiteralFloat 1.7))
  (bind _returnvalue_2 (Math|Random|RandomFloatinRange 1.0 1.0))
  ;[1 1 1 0.5] bubo yelling off of his fucking tiny lungs
  (Utilities|FlowControl|MultiGate true true -1
    (:Out%200
      (Audio|PlaySound2D "/Game/NotFMOD/source/sfx/generic/minigamesGeneral/buboYellingOnTopOfHisLungs/Victory_Bubo_1.Victory_Bubo_1" _returnvalue _returnvalue_2 0.0 0 0))
    (:Out%201
      (Audio|PlaySound2D "/Game/NotFMOD/source/sfx/generic/minigamesGeneral/buboYellingOnTopOfHisLungs/Victory_Bubo_4.Victory_Bubo_4" _returnvalue _returnvalue_2 0.0 0 0))
    (:Out%202
      (Audio|PlaySound2D "/Game/NotFMOD/source/sfx/generic/minigamesGeneral/buboYellingOnTopOfHisLungs/Victory_Bubo_9.Victory_Bubo_9" _returnvalue _returnvalue_2 0.0 0 0))))

(event Custom|generic_beginMinigeim
  ;[1 1 1 0.5] Comment
  (Audio|PlaySound2D "/Game/NotFMOD/source/sfx/generic/ui/begin_minigeim.begin_minigeim" (Math|Float|MakeLiteralFloat 1.0) (Math|Float|MakeLiteralFloat 1.0) 0.0 0 0))

(event Custom|genericBubblePop
  ;[1 1 1 0.5] Comment
  (Audio|PlaySound2D "/Game/NotFMOD/source/sfx/generic/minigamesGeneral/bubblepop.bubblepop" (Math|Float|MakeLiteralFloat 0.8) (Math|Random|RandomFloatinRange 1.0 1.0) 0.0 0 0))

(event Custom|anaPanAway
  ;[1 1 1 0.5] Comment
  (Audio|PlaySound2D "/Game/NotFMOD/source/sfx/minigames/ana/anaPanAway.anaPanAway" (Math|Float|MakeLiteralFloat 1.2) (Math|Random|RandomFloatinRange 1.0 1.0) 0.0 0 0))

(event Custom|ana_button_on
  (Audio|PlaySound2D "/Game/NotFMOD/source/sfx/minigames/ana/ana_button_on.ana_button_on" (Math|Float|MakeLiteralFloat 0.2) (Math|Random|RandomFloatinRange 1.0 1.0) 0.0 0 0)
  (CallFunction|AnaDoorsMoving))

(event Custom|ana_doorsMoving
  (bind _returnvalue (Math|Float|MakeLiteralFloat 0.2))
  (bind _returnvalue_2 (Math|Random|RandomFloatinRange 0.9 1.1))
  ;[1 1 1 0.5] alor alor alor
  (Utilities|FlowControl|MultiGate true true -1
    (:Out%200
      (Audio|PlaySound2D "/Game/NotFMOD/source/sfx/minigames/ana/doorsMoving/ana_doorsMoving_01.ana_doorsMoving_01" _returnvalue _returnvalue_2 0.0 0 0))
    (:Out%201
      (Audio|PlaySound2D "/Game/NotFMOD/source/sfx/minigames/ana/doorsMoving/ana_doorsMoving_02.ana_doorsMoving_02" _returnvalue _returnvalue_2 0.0 0 0))))

(event Custom|ana_button_off
  ;[1 1 1 0.5] Comment
  (Audio|PlaySound2D "/Game/NotFMOD/source/sfx/minigames/ana/ana_button_off.ana_button_off" (Math|Float|MakeLiteralFloat 0.15) (Math|Random|RandomFloatinRange 1.0 1.0) 0.0 0 0)
  (CallFunction|AnaDoorsMoving))

(event Custom|ana_pickTorch
  ;[1 1 1 0.5] Comment
  (Audio|PlaySound2D "/Game/NotFMOD/source/sfx/minigames/ana/anaTorch.anaTorch" (Math|Float|MakeLiteralFloat 1.0) (Math|Random|RandomFloatinRange 0.9 1.1) 0.0 0 0))

(event Custom|ana_AugmentLight
  ;[1 1 1 0.5] Comment
  (Audio|PlaySound2D "/Game/NotFMOD/source/sfx/minigames/ana/anaLightUp.anaLightUp" (Math|Float|MakeLiteralFloat 0.4) (Math|Random|RandomFloatinRange 1.0 1.0) 0.0 0 0))

(event Custom|quino_gudShot
  ;[1 1 1 0.5] Comment
  (Audio|PlaySound2D "/Game/NotFMOD/source/sfx/minigames/quino/quinoGud.quinoGud" (Math|Float|MakeLiteralFloat 1.0) (Math|Random|RandomFloatinRange 1.0 1.0) 0.0 0 0))

(event Custom|quino_midShot
  ;[1 1 1 0.5] Comment
  (Audio|PlaySound2D "/Game/NotFMOD/source/sfx/minigames/quino/quinoMid.quinoMid" (Math|Float|MakeLiteralFloat 0.7) (Math|Float|MakeLiteralFloat 0.9) 0.0 0 0))

(event Custom|quinoBadShot
  ;[1 1 1 0.5] Comment
  (Audio|PlaySound2D "/Game/NotFMOD/source/sfx/minigames/quino/quinoBad.quinoBad" (Math|Float|MakeLiteralFloat 0.7) (Math|Float|MakeLiteralFloat 0.6) 0.0 0 0))

(fn ConstructionScript)