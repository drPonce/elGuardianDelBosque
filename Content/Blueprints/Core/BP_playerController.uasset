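; Player controller that manages UI and minigame logic for the character levels and final exam.
; BeginPlay adds the HUD and a level-specific minigame widget chosen by level name, then overlays a difficulty chooser outside exam and default levels.
; Mateo's minigame loops a pitched beep with difficulty-scaled delays that open timing windows, grading color-matched kicks via debug prints.
; Liu's handlers are empty stubs; a separate event opens the pause menu.
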(event Custom|openPauseMenu
  ;[1 0 0.8395 0.5] pause menu pressed
  (bind _returnvalue (UserInterface|CreateWidget "/Game/Blueprints/Widgets/UI_pauseMenu.UI_pauseMenu_C"))
  (UserInterface|Viewport|AddtoViewport _returnvalue 0))

(event Input|EnhancedActionEvents|EnhancedInputActionIA_touch
  (params (ActionValue :type Vector%202D%20Structure) (ElapsedSeconds :type Float%20%28double-precision%29) (TriggeredSeconds :type Float%20%28double-precision%29) (InputAction :type Input%20Action%20Object%20Reference :default "/Game/Blueprints/Input/Actions/IA_touch.IA_touch"))
  ;[1 0 0.6633 0.5] mouse up and down
  (:Completed
    (switch Utilities|FlowControl|Switch|SwitchonlevelNames (Variables|Default|GetcurrentLevel)
      (:NewEnumerator1
        (CallFunction|MouseUpLiu)))))

(event EventBeginPlay
  ;[1 0.3859 0 0.5] begin play
  (Utilities|FlowControl|Sequence
    (:then_0
      (Input|EnableInput (Game|GetPlayerController 0)))
    (:then_1
      (bind _returnvalue (UserInterface|CreateWidget "/Game/Blueprints/Widgets/UI_HUD.UI_HUD_C"))
      (UserInterface|Viewport|AddtoViewport _returnvalue 0)
      ;;[1 0 0.04507 0.5] create the choose difficulty but dont add it to viewport yet
      (bind _returnvalue_2 (UserInterface|CreateWidget "/Game/Blueprints/Widgets/UI_chooseDifficulty.UI_chooseDifficulty_C"))
      (Variables|components|SetchooseDiff_UI_reference _returnvalue_2))
    (:then_2
      ;;[1 0.5152 0 0.5] open ui depending on current level
      (Utilities|FlowControl|Sequence
        (:then_0
          (bind _returnvalue_3 (Game|GetCurrentLevelName true))
          (switch name (Utilities|String|StringToName _returnvalue_3)
            (:LVL_quino
              (bind _returnvalue_4 (UserInterface|CreateWidget "/Game/Blueprints/Widgets/minigames/quino/UI_quino.UI_quino_C"))
              (bind _output_get (Variables|components|Setminigame_UI_reference _returnvalue_4))
              (UserInterface|Viewport|AddtoViewport _output_get 0)
              (Rendering|Components|TextRender|SetText (Variables|/Game/Blueprints/Widgets/UI_chooseDifficulty.UI_chooseDifficulty_C|GetlevelTitleText (Variables|components|GetchooseDiff_UI_reference)) "Quino's Level")
              (Variables|Default|SetcurrentLevel "NewEnumerator0"))
            (:LVL_mateo
              (bind _returnvalue_5 (UserInterface|CreateWidget "/Game/Blueprints/Widgets/minigames/mateo/UI_mateo.UI_mateo_C"))
              (bind _output_get_2 (Variables|components|Setminigame_UI_reference _returnvalue_5))
              (UserInterface|Viewport|AddtoViewport _output_get_2 0)
              (Rendering|Components|TextRender|SetText (Variables|/Game/Blueprints/Widgets/UI_chooseDifficulty.UI_chooseDifficulty_C|GetlevelTitleText (Variables|components|GetchooseDiff_UI_reference)) "Mateo's Level")
              (Variables|Default|SetcurrentLevel "NewEnumerator3"))
            (:LVL_ana
              (bind _returnvalue_6 (UserInterface|CreateWidget "/Game/Blueprints/Widgets/minigames/ana/UI_ana.UI_ana_C"))
              (bind _output_get_3 (Variables|components|Setminigame_UI_reference _returnvalue_6))
              (UserInterface|Viewport|AddtoViewport _output_get_3 0)
              (Rendering|Components|TextRender|SetText (Variables|/Game/Blueprints/Widgets/UI_chooseDifficulty.UI_chooseDifficulty_C|GetlevelTitleText (Variables|components|GetchooseDiff_UI_reference)) "Ana's Level")
              (Variables|Default|SetcurrentLevel "NewEnumerator2"))
            (:LVL_liu
              (bind _returnvalue_7 (UserInterface|CreateWidget "/Game/Blueprints/Widgets/minigames/liu/UI_liu.UI_liu_C"))
              (bind _output_get_4 (Variables|components|Setminigame_UI_reference _returnvalue_7))
              (UserInterface|Viewport|AddtoViewport _output_get_4 0)
              (Rendering|Components|TextRender|SetText (Variables|/Game/Blueprints/Widgets/UI_chooseDifficulty.UI_chooseDifficulty_C|GetlevelTitleText (Variables|components|GetchooseDiff_UI_reference)) "Liu's Level")
              (Variables|Default|SetcurrentLevel "NewEnumerator1"))
            (:LVL_finalExam
              (bind _returnvalue_8 (UserInterface|CreateWidget "/Game/Blueprints/Widgets/minigames/finalExam/UI_finalExam.UI_finalExam_C"))
              (bind _output_get_5 (Variables|components|Setminigame_UI_reference _returnvalue_8))
              (UserInterface|Viewport|AddtoViewport _output_get_5 0)
              (Variables|Default|SetcurrentLevel "NewEnumerator4"))
            (:LVL_defaultLevel
              (Variables|Default|SetcurrentLevel "NewEnumerator5"))))
        (:then_1
          (if (and (!= (Utilities|String|StringToName _returnvalue_3) "LVL_finalExam") (!= (Utilities|String|StringToName _returnvalue_3) "LVL_defaultLevel"))
            ;;;[1 0 0.01209 0.5] now you can add to viewport, on top of the other one
            (Utilities|IsValid (Variables|components|GetchooseDiff_UI_reference)
              (:Is%20Valid
                (UserInterface|Viewport|AddtoViewport (Variables|components|GetchooseDiff_UI_reference) 0)))))))))

(event Custom|beginFunctionsMateo
  (params (difficultyIndex :type Integer))
  ;[1 0.5436 0 0.5] begin functions
  (Utilities|FlowControl|Sequence
    (:then_0
      (Development|PrintString "Good luck! get ready" true true "(R=0.000000,G=0.660000,B=1.000000,A=1.000000)" 3.0)
      (Development|PrintString "Press the interact button right before the final beep sounds " true true "(R=0.000000,G=0.660000,B=1.000000,A=1.000000)" 3.0)
      (Development|PrintString (Utilities|String|Append "Difficulty set to " (Utilities|String|ToString(Integer) difficultyIndex)) true true "(R=0.000000,G=0.660000,B=1.000000,A=1.000000)" 3.0)
      (Utilities|FlowControl|Delay 3.0)
      (CallFunction|BeginShotTimeline))
    (:then_1
      (bind _asui_mateo (Utilities|Casting|CastToUI_mateo (Variables|components|Getminigame_UI_reference)))
      (Variables|Components|SetPelouti (Variables|/Game/Blueprints/Widgets/minigames/mateo/UI_mateo.UI_mateo_C|Getpelouti _asui_mateo))
      (Variables|Default|SetcurrentDifficultyIndex difficultyIndex) ; lo necesitamos tener a mano siempre
    )))

(event Custom|shotTimeline_steps
  ;[0.9558 0.6312 1 0.5] shot timeline
  (Utilities|FlowControl|Sequence
    (:then_0
      (Variables|mateo|SetballTimeGaps "NewEnumerator1"))
    (:then_1
      (Utilities|FlowControl|Delay (- (Variables|Mateo|GettimeUntilBeep) (Variables|Mateo|GetmidShotThreshold)))
      (Variables|mateo|SetballTimeGaps "NewEnumerator2"))
    (:then_2
      (Utilities|FlowControl|Delay (- (Variables|Mateo|GettimeUntilBeep) (Variables|Mateo|GetperfShotThreshold)))
      (Variables|mateo|SetballTimeGaps "NewEnumerator3")
      (Development|PrintString "Hello"))
    (:then_3
      (Utilities|FlowControl|Delay (+ (Variables|Mateo|GettimeUntilBeep) (Variables|Mateo|GetperfShotThreshold)))
      (Variables|mateo|SetballTimeGaps "NewEnumerator2"))
    (:then_4
      (Utilities|FlowControl|Delay (+ (Variables|Mateo|GettimeUntilBeep) (Variables|Mateo|GetmidShotThreshold)))
      (Variables|mateo|SetballTimeGaps "NewEnumerator1"))
    (:then_5
      (Utilities|FlowControl|Delay (+ (Variables|Mateo|GettimeUntilBeep) 2.0))
      (Variables|mateo|SetballTimeGaps "NewEnumerator0"))))

(event Custom|mateoKickButtonPressed
  (params (colorIndex :type Integer))
  ;[1 0 0.9086 0.5] playerKickedTheBall
  (if (Utilities|Enum|NotEqual(Enum) (Variables|mateo|GetballTimeGaps) "NewEnumerator0") ; if we are not counting, ignore\nit and do nothing
    (if (== colorIndex (Variables|Mateo|GetcurrentBallColorIndex)) ; is the player pressing\nthe correct color?\nif not its an automatic\nbad
      (switch Utilities|FlowControl|Switch|SwitchonmateoTimeGaps (Variables|mateo|GetballTimeGaps)
        (:NewEnumerator1
          (Development|PrintString "YOU FUCKING SUCK" :!label _label))
        (:NewEnumerator2
          (Development|PrintString "YOU ARE MEDIOCRE"))
        (:NewEnumerator3
          (Development|PrintString "you are allright i guess")))
      (else
        (goto _label)))))

(event Custom|beginShotTimeline
  (bind _pelouti (Variables|Components|GetPelouti))
  ;[0.9618 0.545 1 0.5] begin shot timeline
  (Development|PrintString "Go!")
  (Audio|PlaySound2D "/Game/Testing/testingSounds/horrorBeep.horrorBeep" 1.0 (Utilities|Select :Index (Variables|Default|GetcurrentDifficultyIndex) :Option%200 0.0 :Option%201 0.87 :Option%202 1.33 :Option%203 1.8) 0.0 0 0)
  (Variables|Mateo|SettimeUntilBeep (Utilities|Select :Index (Variables|Default|GetcurrentDifficultyIndex) :Option%200 0.0 :Option%201 1.9 :Option%202 1.4 :Option%203 1.15))
  (bind _output_get (Variables|Mateo|SetcurrentBallColorIndex (Utilities|Select :Index (Variables|Default|GetcurrentDifficultyIndex) :Option%200 0 :Option%201 1 :Option%202 (Math|Random|RandomIntegerinRange 1 2) :Option%203 (Math|Random|RandomIntegerinRange 1 4))))
  (Utilities|IsValid _pelouti
    (:Is%20Valid
      (Class|Image|SetBrushTintColor _pelouti (Utilities|Select :Index _output_get :Option%200 "" :Option%201 (Utilities|Struct|MakeSlateColor "(R=1.000000,G=0.181164,B=0.904661,A=1.000000)") :Option%202 (Utilities|Struct|MakeSlateColor "(R=0.000000,G=0.577581,B=1.000000,A=1.000000)") :Option%203 (Utilities|Struct|MakeSlateColor "(R=0.346704,G=1.000000,B=0.351533,A=1.000000)") :Option%204 (Utilities|Struct|MakeSlateColor "(R=1.000000,G=1.000000,B=1.000000,A=1.000000)")))
      (CallFunction|ShotTimelineSteps)
      (Utilities|FlowControl|Delay (Utilities|Select :Index (Variables|Default|GetcurrentDifficultyIndex) :Option%200 0.0 :Option%201 4.0 :Option%202 3.0 :Option%203 2.5))
      (CallFunction|BeginShotTimeline) ; loop it
    )))

(event Custom|CustomEvent
  (params (difficultyIndex :type Integer))
  ;[1 1 1 0.5] begin functions liu
  (Utilities|FlowControl|Sequence))

(event Custom|interactButtonPressed)

(event Custom|mouseUpLiu)

(fn ConstructionScript)