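; BP_universalInfo is a core Blueprint that blacks out the player camera at initialization.
; Init runs a near-instant camera fade to full opacity and holds it, while createHUD only triggers a DoOnce with nothing after it.
; Unconnected leftovers hold a testing bypass for the loading screen, noted as formerly in the player controller, and creation of the UI_ana widget.
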(event Custom|createHUD
  (Utilities|FlowControl|DoOnce false))

(event EventInit
  (CameraFades|StartCameraFade :self (Game|GetPlayerCameraManager 0) :ToAlpha 1.0 :Duration 0.001 :bHoldWhenFinished true))